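; Enemy Blueprint that attacks by launching a catching hand (a CathHand child actor) toward the player.
; While the attack flag is set and it is alive, a delay timer triggers the montage and locks the direction to the player's current position.
; Tick moves the hand along that line until it exceeds maximum reach or reports a catch, then returns it to its launch point and stops it.
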(event `self.ReceiveBeginPlay`
  (`parent.ReceiveBeginPlay`))

(event `self.ReceiveTick`
  (params (DeltaSeconds :type "Float (single-precision)"))
  (bind _attackdelay (`self.AttackDelay`))
  (bind _childactor (`ChildActorComponent.ChildActor` (`self.ChildActor`)))
  (bind _childactor_2 (`ChildActorComponent.ChildActor` (`self.ChildActor`)))
  (bind _childactor_3 (`ChildActorComponent.ChildActor` (`self.ChildActor`)))
  (bind _returnvalue (`self.K2_GetActorLocation` (`ChildActorComponent.ChildActor` (`self.ChildActor`))))
  (`parent.ReceiveTick` DeltaSeconds)
  (`|ExecutionSequence`
    (:`then_0`
      (if (and (`self.AttackFLag`) (not (`self.Death`)))
        (if (<= _attackdelay 0.0)
          (bind _returnvalue_2 (`self.PlayAnimMontage` "/Game/Animations/Enemy/LongDis/LongAttack_Montage.LongAttack_Montage" 1.0 "Default"))
          (set `self.AttackDelay` (+ _returnvalue_2 (`self.MaxAttackDelay`)))
          (set `self.CathingFlag` true)
          (set `self.StartLocation` (`self.K2_GetActorLocation` (`ChildActorComponent.ChildActor` (`self.ChildActor`))))
          (set `self.ReturnValue` (* (`KismetMathLibrary.Normal` (- (`self.K2_GetActorLocation` (`GameplayStatics.GetPlayerCharacter` 0)) (`self.StartLocation`))) (`self.speed`)))
          (bind _ascath_hand (cast `/Game/BP/Enemy/Catch/CathHand` (`ChildActorComponent.ChildActor` (`self.ChildActor`))))
          (set `/Game/BP/Enemy/Catch/CathHand.StopHand` false _ascath_hand)
          (set `/Game/BP/Enemy/Catch/CathHand.CathFlag` false _ascath_hand)
          (set `self.MoveAndReturnFlag` false)
          (else
            (set `self.AttackDelay` (- _attackdelay DeltaSeconds))))))
    (:`then_1`
      (if (and (< (`self.AttackDelay`) 0.0) (`self.AttackFLag`))
        (set `self.AttackFLag` false)))
    (:`then_2`
      (if (`self.CathingFlag`)
        (if (`self.MoveAndReturnFlag`)
          (`self.K2_SetActorLocation` _childactor_3 (+ _returnvalue (* (`KismetMathLibrary.Normal` (- (`self.StartLocation`) (`self.K2_GetActorLocation` (`ChildActorComponent.ChildActor` (`self.ChildActor`))))) (`self.speed`))) false false)
          (if (< (`KismetMathLibrary.Vector_Distance` (`self.K2_GetActorLocation` _childactor_3) (`self.StartLocation`)) 50.0)
            (set `self.CathingFlag` false)
            (set `self.MoveAndReturnFlag` false)
            (set `self.ReturnValue` (0.0 0.0 0.0))
            (`self.K2_SetActorLocation` _childactor (`self.StartLocation`) false false)
            (bind _ascath_hand_2 (cast `/Game/BP/Enemy/Catch/CathHand` _childactor))
            (set `/Game/BP/Enemy/Catch/CathHand.StopHand` true _ascath_hand_2))
          (else
            (`self.K2_SetActorLocation` _childactor_2 (+ _returnvalue (`self.ReturnValue`)) false false)
            (if (> (`KismetMathLibrary.Vector_Distance` (`self.K2_GetActorLocation` _childactor_2) (`self.StartLocation`)) (`self.MaxCathLength`))
              (set `self.MoveAndReturnFlag` true)
              (set `self.ReturnValue` (`self.ReturnValue`)))))))
    (:`then_3`
      (bind _ascath_hand_3 (cast `/Game/BP/Enemy/Catch/CathHand` (`ChildActorComponent.ChildActor` (`self.ChildActor`))))
      (if (`/Game/BP/Enemy/Catch/CathHand.CathFlag` _ascath_hand_3)
        (set `self.MoveAndReturnFlag` true)
        (set `self.ReturnValue` (`self.ReturnValue`))))))

(fn `UserConstructionScript`
  (`parent.UserConstructionScript`))