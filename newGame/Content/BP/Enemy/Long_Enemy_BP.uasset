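; Ranged enemy Blueprint that fires EnemyBullet projectiles while its attack flag is set and it is not dead.
; Tick runs a cooldown; when it expires, the enemy plays LongAttack_Montage and sets the delay to montage length plus a pause.
; Each bullet spawns at BulletPos with the actor's rotation, marked non-friendly and given the shooter's location.
; Tick clears the attack flag once the cooldown drops below zero; nothing here sets it.
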(event `self.ReceiveTick`
  (params (DeltaSeconds :type "Float (single-precision)"))
  (bind (_returnvalue_location _returnvalue_rotation _returnvalue_scale) (`KismetMathLibrary.BreakTransform` (`self.GetTransform`)))
  (bind _attackdelay (`self.AttackDelay`))
  (`parent.ReceiveTick` DeltaSeconds)
  (`|ExecutionSequence`
    (:`then_0`
      (if (and (`self.AttackFLag`) (not (`self.Death`)))
        (if (<= _attackdelay 0.0)
          (bind _returnvalue (`self.PlayAnimMontage` "/Game/Animations/Enemy/LongDis/LongAttack_Montage.LongAttack_Montage" 1.0 "Default"))
          (set `self.AttackDelay` (+ _returnvalue 1.0))
          (bind _returnvalue_2 (`|SpawnActorFromClass` "/Game/BP/Enemy/EnemyBullet.EnemyBullet_C" (`KismetMathLibrary.MakeTransform` (`SceneComponent.K2_GetComponentLocation` (`self.bulletPos`)) _returnvalue_rotation _returnvalue_scale) "Undefined" "OverrideRootScale" null null))
          (set `/Game/BP/Enemy/EnemyBullet.Friendship` false _returnvalue_2)
          (set `/Game/BP/Enemy/EnemyBullet.EnemyPos` (`self.K2_GetActorLocation`) _returnvalue_2)
          (else
            (set `self.AttackDelay` (- _attackdelay DeltaSeconds))))))
    (:`then_1`
      (if (and (< (`self.AttackDelay`) 0.0) (`self.AttackFLag`))
        (set `self.AttackFLag` false)))))

(fn `UserConstructionScript`
  (`parent.UserConstructionScript`))