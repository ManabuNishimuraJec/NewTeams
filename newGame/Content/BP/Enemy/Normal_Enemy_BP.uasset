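; Normal enemy Blueprint that adds a timed melee-or-similar attack montage on top of its parent's Tick logic.
; While AttackFLag is set and neither Death nor DontAttack blocks it, Tick plays Enemy_Attack or counts AttackDelay down.
; The cooldown equals the montage length plus a one-second pause, and AttackFLag clears once it drops below zero.
; Nothing in this file sets AttackFLag to true.
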(event `self.ReceiveTick`
  (params (DeltaSeconds :type "Float (single-precision)"))
  (bind _attackdelay (`self.AttackDelay`))
  (`parent.ReceiveTick` DeltaSeconds)
  (`|ExecutionSequence`
    (:`then_0`
      (if (and (`self.AttackFLag`) (not (`self.Death`)) (not (`self.DontAttack`)))
        (if (<= _attackdelay 0.0)
          (bind _returnvalue (`self.PlayAnimMontage` "/Game/BP/Enemy/Enemy_Attack.Enemy_Attack" 1.0 "Default"))
          (set `self.AttackDelay` (+ _returnvalue 1.0))
          (else
            (set `self.AttackDelay` (- _attackdelay DeltaSeconds))))))
    (:`then_1`
      (if (and (< (`self.AttackDelay`) 0.0) (`self.AttackFLag`))
        (set `self.AttackFLag` false)))))

(fn `UserConstructionScript`
  (`parent.UserConstructionScript`))