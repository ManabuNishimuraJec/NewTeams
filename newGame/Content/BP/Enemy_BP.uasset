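; Enemy character Blueprint that handles damage, a frightened state and death.
; Hits from a BaseWeapon whose type matches the enemy's Attribute build points until they trigger the frightened flag in Enemy_Anime_Bp.
; Tick times out that animation flag, while other non-lethal hits play a hit montage and clear the state.
; At zero health it runs a one-time montage call, pauses mesh animation just before the end and disables movement.
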(event `self.ReceiveTick`
  (params (DeltaSeconds :type "Float (single-precision)"))
  (if (`self.FrigFlag`)
    (set `self.FrightenedPoint` 0)
    (set `self.Timer` (+ (`self.Timer`) DeltaSeconds))
    (if (>= (`self.Timer`) (`self.MaxFrigTimer`))
      (bind _asenemy_anime_bp (cast `/Game/Animations/Enemy/Enemy_Anime_Bp` (`SkeletalMeshComponent.GetAnimInstance` (`self.Mesh`))))
      (set `/Game/Animations/Enemy/Enemy_Anime_Bp.Frightened` false _asenemy_anime_bp))))

(event `self.ReceiveAnyDamage`
  (params (Damage :type "Float (single-precision)") (DamageType :type "DamageType Object Reference") (InstigatedBy :type "Controller Object Reference") (DamageCauser :type "Actor Object Reference"))
  (bind _returnvalue (`SkeletalMeshComponent.GetAnimInstance` (`self.Mesh`)))
  (bind _returnvalue_2 (>= (`self.FrightenedPoint`) (`self.MaxFrigPoint`)))
  ;[1 1 1] 攻撃を受けた場合の処理
  (bind _asbase_weapon (cast `/Game/BP/BaseWeapon` DamageCauser))
  (if (== (`KismetMathLibrary.Conv_ByteToInt` (`self.Attribute`)) (`KismetMathLibrary.Conv_ByteToInt` (`/Game/BP/BaseWeapon.weaponType` _asbase_weapon)))
    (`KismetSystemLibrary.PrintString` "onaji")
    (`/Engine/EditorBlueprintResources/StandardMacros.IncrementInt` (`self.FrightenedPoint`)
      (:`  `
        _)))
  (bind _output_get (set `self.health` (- (`self.health`) Damage)))
  (if (> _output_get 0.0)
    (if (and _returnvalue_2 (not (`self.FrigFlag`)))
      (set `self.FrigFlag` _returnvalue_2)
      (bind _asenemy_anime_bp (cast `/Game/Animations/Enemy/Enemy_Anime_Bp` _returnvalue))
      (set `/Game/Animations/Enemy/Enemy_Anime_Bp.Frightened` true _asenemy_anime_bp)
      (set `self.Timer` 0.0)
      (set `self.FrightenedPoint` 0)
      (else
        ;;[1 1 1] HPがまだ残っている状態
        (`self.PlayAnimMontage` "/Game/Animations/Enemy/Hit/Getting_Hit_mixamo_com_Montage.Getting_Hit_mixamo_com_Montage")
        (bind _asenemy_anime_bp_2 (cast `/Game/Animations/Enemy/Enemy_Anime_Bp` _returnvalue))
        (set `/Game/Animations/Enemy/Enemy_Anime_Bp.Frightened` false _asenemy_anime_bp_2)
        (set `self.Timer` 0.0)
        (set `self.FrigFlag` false)))
    (else
      ;;[1 1 1] 死んだ時
      (`/Engine/EditorBlueprintResources/StandardMacros.DoOnce` false
        (:`Completed`
          (bind _returnvalue_3 (`self.PlayAnimMontage` null))
          (`KismetSystemLibrary.Delay` (- _returnvalue_3 0.27))
          (set `SkeletalMeshComponent.bPauseAnims` true (`self.Mesh`))
          (`CharacterMovementComponent.DisableMovement` (`self.CharacterMovement`)))))))

(fn `UserConstructionScript`)