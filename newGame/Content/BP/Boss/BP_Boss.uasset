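; Boss character that fights the player with dodges, a melee combo and three montage-driven ranged attacks spawned on anim notifies.
; A Tick sequence drives behavior from distance bands, timers, damage taken and player attacks, triggering random dodges, counters and escapes.
; Timed attacks pass through RandAttackChoice, meant to avoid repeats and cap low and medium picks.
; BeginPlay handles second-phase transition effects, while the second-phase special move is unwired.
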(event `dodge`
  (set `self.dodgeFlag` true)
  (`self.K2_SetActorRotation` (`KismetMathLibrary.FindLookAtRotation` (`self.K2_GetActorLocation`) (`self.K2_GetActorLocation` (`GameplayStatics.GetPlayerPawn` 0))))
  (`|PlayMontage` (`self.Mesh`) "/Game/BP/Boss/MagicalAnimSet/Animations/dodge/RootMotion/dodge_b_Montage.dodge_b_Montage"
    (:`OnCompleted`
      (set `self.dodgeFlag` false))))

(event `self.ReceiveTick`
  (params (DeltaSeconds :type "Float (single-precision)"))
  (`|ExecutionSequence`
    (:`then_0`
      (if (`self.lookFlag`)
        (`self.K2_SetActorRotation` (`KismetMathLibrary.FindLookAtRotation` (`self.K2_GetActorLocation`) (`self.K2_GetActorLocation` (`GameplayStatics.GetPlayerPawn` 0))))))
    (:`then_1`
      (set `self.Delta Seconds` DeltaSeconds)
      (`|ExecutionSequence`
        (:`then_0`
          ;[1 1 1] 距離チェック
          (bind _output_get (set `self.CheckDisTime` (+ (`self.CheckDisTime`) 1.0)))
          (if (> _output_get 30.0)
            (set `self.CheckDisTime` 0.0)
            (bind _approach (`self.CheckPlayerDIstance`))
            (set `self.ApproachFlag` _approach)
            (`self.SetPlayerDistance`)))
        (:`then_1`
          ;[1 1 1] ドッジ判定
          (if (and (not (`self.isAttack`)) (not (`self.dodgeFlag`)) (not (`self.isMove`)))
            (if (`self.ApproachFlag`)
              (switch `int` (`KismetMathLibrary.RandomInteger` 6)
                (:`Default`
                  (set `self.ApproachFlag` false))
                (:`0`
                  (set `self.ApproachFlag` false)
                  (`self.dodge`))))))
        (:`then_2`
          ;[1 1 1] Counter攻撃
          (switch `/Game/BP/Boss/POSITION_NUM` (`self.NowDisPos`)
            (:`NewEnumerator0`
              (if (not (`self.isAttack`))
                (bind _ascharactor_bp (cast `/Game/BP/Charactor_BP` (`GameplayStatics.GetPlayerPawn` 0)))
                (bind _isattack (`/Game/BP/Charactor_BP.GetPlayerAttack` _ascharactor_bp))
                (if _isattack
                  (if (`self.CounterCheck`)
                    (bind _result (`/Engine/EditorBlueprintResources/StandardMacros.IncrementFloat` (`self.nextCounterTime`))
                      (:`  `
                        (if (>= _result 60.0)
                          (set `self.nextCounterTime` 0.0)
                          (`/Engine/EditorBlueprintResources/StandardMacros.DoOnce` false :!label _label
                            (:`Completed`
                              (if (not (`self.isDamage`))
                                (switch `int` (`KismetMathLibrary.RandomInteger` 3)
                                  (:`Default`
                                    (set `self.CounterCheck` true)
                                    (`self.CounterCheck＿event`))
                                  (:`0`
                                    (if (not (`self.isAttack`))
                                      (`self.Attack`))))))))))
                    (else
                      (goto _label)))
                  (else
                    (set `self.CounterCheck` false)
                    (goto _label :!via `Reset`)))))))
        (:`then_3`
          ;[1 1 1] ダメージフラグリセット
          (if (`self.isDamage`)
            (bind _output_get_2 (set `self.DamageTime` (+ (`self.DamageTime`) (`self.Delta Seconds`))))
            (if (>= _output_get_2 0.3)
              (set `self.isDamage` false)
              (set `self.DamageTime` 0.0))))
        (:`then_4`
          ;[1 1 1] Hit8秒後に攻撃
          (if (`self.hitFlag`)
            (bind _output_get_3 (set `self.hitTimer` (+ (`self.hitTimer`) (`self.Delta Seconds`))))
            (if (>= _output_get_3 8.0)
              (set `self.hitTimer` 0.0)
              (if (not (`self.isAttack`))
                (set `self.hitFlag` false)
                (switch `int` (`KismetMathLibrary.RandomInteger` 3)
                  (:`0`
                    (set `self.isAttack` true)
                    (set `self.counterAttack` true))
                  (:`1`
                    (`self.dodge`)
                    (`KismetSystemLibrary.Delay` 1.2)
                    (set `self.isAttack` true)
                    (`self.StartMediumAttack`))
                  (:`2`
                    (set `self.isAttack` true)
                    (`self.StartHeighAttack`)))))))
        (:`then_5`
          ;[1 1 1] ブロックチェック
          (bind _ascharactor_bp_2 (cast `/Game/BP/Charactor_BP` (`GameplayStatics.GetPlayerPawn` 0)))
          (if (and (>= (`/Game/BP/Charactor_BP.BlockNowTime` _ascharactor_bp_2) 5.0) (not (`self.BlockCheckFlag`)))
            (switch `int` (`KismetMathLibrary.RandomInteger` 3)
              (:`Default`
                (set `/Game/BP/Charactor_BP.BlockNowTime` 0.0 _ascharactor_bp_2))
              (:`0`
                (set `self.BlockCheckFlag` true)
                (set `/Game/BP/Charactor_BP.BlockNowTime` 0.0 _ascharactor_bp_2)))))
        (:`then_6`
          ;[1 1 1] 1.5割消費時dodge
          (bind _result_2 (`/Engine/EditorBlueprintResources/StandardMacros.IncrementFloat` (`self.CheckTime`))
            (:`  `
              (if (> _result_2 300.0)
                (if (>= (* (/ (- (`self.CHeckHp`) (`self.HP`)) (`self.CHeckHp`)) 100.0) 1.5)
                  (set `self.escapeFLag` true)
                  (set `self.CHeckHp` (`self.HP`)))))))
        (:`then_7`
          (if (`self.escapeFLag`)
            (`/Engine/EditorBlueprintResources/StandardMacros.DoOnce` false :!label _label_2
              (:`Completed`
                (switch `/Game/BP/Boss/POSITION_NUM` (`self.NowDisPos`)
                  (:`NewEnumerator0`
                    (`self.dodge`)
                    (`KismetSystemLibrary.Delay` 1.0)
                    (`self.SetPlayerDistance`)
                    (switch `/Game/BP/Boss/POSITION_NUM` (`self.NowDisPos`)
                      (:`NewEnumerator0`
                        (`self.nextDodge` :!label _label_3))
                      (:`NewEnumerator1`
                        (set `self.escapeFLag` false :!label _label_4))
                      (:`NewEnumerator2`
                        (goto _label_4))))
                  (:`NewEnumerator1`
                    (`self.dodge`)
                    (`KismetSystemLibrary.Delay` 1.0)
                    (`self.SetPlayerDistance`)
                    (switch `/Game/BP/Boss/POSITION_NUM` (`self.NowDisPos`)
                      (:`NewEnumerator0`
                        (goto _label_3))
                      (:`NewEnumerator1`
                        (goto _label_3))
                      (:`NewEnumerator2`
                        (set `self.escapeFLag` false)))))))))
        (:`then_8`
          ;[1 1 1] 移動処理
          (if (and (not (`self.isAttack`)) (not (`self.dodgeFlag`)) (not (`self.isMove`)))
            (`/Engine/EditorBlueprintResources/StandardMacros.IncrementFloat` (`self.MoveCheckTime`)
              (:`  `
                (if (>= (`self.MoveCheckTime`) 600.0)
                  (set `self.moveCheckFlag` true)
                  (set `self.MoveCheckTime` 0.0))))))
        (:`then_9`
          (if (!= (`KismetMathLibrary.VSizeSquared` (`self.GetVelocity`)) 0.0)
            (set `self.isMove` true)
            (else
              (set `self.isMove` false))))
        (:`then_10`
          (if (not (`self.isAttack`))
            (bind _output_get_4 (set `self.AttackTime` (+ (`self.AttackTime`) (`self.Delta Seconds`))))
            (if (>= _output_get_4 10.0)
              (`/Engine/EditorBlueprintResources/StandardMacros.DoOnce` false :!label _label_5
                (:`Completed`
                  (bind _attacknum (`self.RandAttackChoice`))
                  (switch `int` _attacknum
                    (:`0`
                      (`self.StartLowAttack`))
                    (:`1`
                      (`self.StartMediumAttack`))
                    (:`2`
                      (`self.StartHeighAttack`))))))))))))

(event `Attack`
  (set `self.isAttack` true)
  (`|PlayMontage` (`self.Mesh`) "/Game/BP/Boss/MagicalAnimSet/Animations/attack/13_basiccombo/Combo_fast.Combo_fast"
    (:`OnCompleted`
      (set `self.isAttack` false))))

(event `AttackENd`
  (set `self.AttackTime` 0.0)
  (set `self.lookFlag` false)
  (set `self.isAttack` false)
  (`self.AttackReset`))

(event `CounterCheck＿event`
  ;[1 1 1] Counter攻撃
  (goto _label :!via `Reset`))

(event `StartLowAttack`
  (bind (_returnvalue_roll _returnvalue_pitch _returnvalue_yaw) (`KismetMathLibrary.BreakRotator` (`self.K2_GetActorRotation`)))
  (bind _returnvalue (`SceneComponent.K2_GetComponentLocation` (`self.shotPos`)))
  (bind _returnvalue_2 (+ _returnvalue_pitch -5.0))
  (`self.ToPlayerDir`)
  ;[1 1 1] 球状の飛び道具を3回飛ばす：攻撃頻度「高」
  (bind _notifyname (`|PlayMontage` (`self.Mesh`) "/Game/BP/Boss/MagicalAnimSet/Animations/attack/02_shot/02_shot_all.02_shot_all")
    (:`then`
      (set `self.lookFlag` true))
    (:`OnCompleted`
      (`self.AttackENd`)
      (`KismetSystemLibrary.Delay` 1.0))
    (:`OnNotifyBegin`
      (switch `name` _notifyname
        (:`Shot`
          (`|SpawnActorFromClass` "/Game/BP/Boss/shot1.shot1_C" (`KismetMathLibrary.MakeTransform` _returnvalue (`KismetMathLibrary.MakeRotator` _returnvalue_roll _returnvalue_2 _returnvalue_yaw)) "Undefined" "OverrideRootScale" null null))
        (:`LastShot`
          (bind _returnvalue_3 (`|SpawnActorFromClass` "/Game/BP/Boss/shot1.shot1_C" (`KismetMathLibrary.MakeTransform` _returnvalue (`KismetMathLibrary.MakeRotator` _returnvalue_roll _returnvalue_2 _returnvalue_yaw)) "Undefined" "OverrideRootScale" null null))
          (`/Game/BP/Boss/shot1.SetLastShot` _returnvalue_3))))))

(event `ToPlayerDir`
  (`self.K2_SetActorRotation` (`KismetMathLibrary.FindLookAtRotation` (`self.K2_GetActorLocation`) (`self.K2_GetActorLocation` (`GameplayStatics.GetPlayerPawn` 0)))))

(event `StartMediumAttack`
  (`self.ToPlayerDir`)
  ;[1 1 1] 円柱型の遠距離攻撃：攻撃頻度「低」
  (bind _notifyname (`|PlayMontage` (`self.Mesh`) "/Game/BP/Boss/MagicalAnimSet/Animations/attack/04_beam/Inplace/04_beam_all.04_beam_all")
    (:`OnCompleted`
      (`self.AttackENd`))
    (:`OnNotifyBegin`
      (switch `name` _notifyname
        (:`shot`
          (bind _returnvalue (`|SpawnActorFromClass` "/Game/BP/Boss/Shot2.Shot2_C" (`KismetMathLibrary.MakeTransform` (`SceneComponent.K2_GetComponentLocation` (`self.shotPos`)) (`SceneComponent.K2_GetComponentRotation` (`self.CapsuleComponent`))) "Undefined" "OverrideRootScale" null null))
          (set `self.Bream2` _returnvalue))
        (:`shotEnd`
          (`self.K2_DestroyActor` (`self.Bream2`)))))))

(event `StartHeighAttack`
  (`self.ToPlayerDir`)
  ;[1 1 1] 半月型の飛び道具を飛ばす：攻撃頻度「中」
  (bind _notifyname (`|PlayMontage` (`self.Mesh`) "/Game/BP/Boss/MagicalAnimSet/Animations/attack/05_chanting/Inplace/05_chanting_all.05_chanting_all")
    (:`OnCompleted`
      (`self.AttackENd`))
    (:`OnNotifyBegin`
      (switch `name` _notifyname
        (:`Shot`
          (`|SpawnActorFromClass` "/Game/BP/Boss/shot3.shot3_C" (`KismetMathLibrary.MakeTransform` (`SceneComponent.K2_GetComponentLocation` (`self.shotPos`))) "Undefined" "OverrideRootScale" null null))
        (:`ShotRight`
          (bind _returnvalue (`|SpawnActorFromClass` "/Game/BP/Boss/shot3.shot3_C" (`KismetMathLibrary.MakeTransform` (`SceneComponent.K2_GetComponentLocation` (`self.shotPos`))) "Undefined" "OverrideRootScale" null null))
          (set `/Game/BP/Boss/shot3.dirRight` true _returnvalue))))))

(event `nextDodge`
  ;[1 1 1] 1.5割消費時dodge
  (goto _label_2 :!via `Reset`))

(event `self.ReceiveAnyDamage`
  (params (Damage :type "Float (single-precision)") (DamageType :type "DamageType Object Reference") (InstigatedBy :type "Controller Object Reference") (DamageCauser :type "Actor Object Reference"))
  (set `self.HP` (- (`self.HP`) Damage))
  (if (> (`self.HP`) 0.0)
    (set `self.isDamage` true)
    (set `self.hitFlag` true)
    (set `self.isAttack` false)
    (`self.PlayAnimMontage` "/Game/BP/Boss/MagicalAnimSet/Animations/damage/Inplace/damage_f_Montage.damage_f_Montage")
    (else
      (`/Engine/EditorBlueprintResources/StandardMacros.DoOnce` false))))

(event `AttackReset`
  (goto _label_5 :!via `Reset`))

(event `Attack_Collision_ON`
  (`PrimitiveComponent.SetCollisionProfileName` (`self.AttackCollision1`) "OverlapAll" true))

(event `Attack_Collision2_On`
  (`PrimitiveComponent.SetCollisionProfileName` (`self.AttackCollision2`) "OverlapAll" true))

(event `Attack_Collision_OFF`
  (`PrimitiveComponent.SetCollisionEnabled` (`self.AttackCollision1`) "NoCollision"))

(event `Attack_Collision2_OFF`
  (`PrimitiveComponent.SetCollisionEnabled` (`self.AttackCollision2`) "NoCollision"))

(event `self.ReceiveBeginPlay`
  ;[1 1 1] 第二形態移行時のエフェクト
  (bind _notifyname (`|PlayMontage` (`self.Mesh`))
    (:`OnNotifyBegin`
      (switch `name` _notifyname
        (:`Effect Start`
          (`|ExecutionSequence`
            (:`then_0`
              (bind _returnvalue (`GameplayStatics.SpawnEmitterAttached` "/Game/Effect/Effects_Boss/FANVFXCollection2/5_ParticleSystem/Buff/Buff_02/P_Buff_02_05.P_Buff_02_05" (`self.CapsuleComponent`) "None" (0.0 0.0 0.0) (struct) (5.0 5.0 5.0))))
            (:`then_1`
              (bind (_direction `_新規track_0`) (`Timeline|タイムライン_0` :!via `PlayFromStart`)
                (:`Update`
                  (`SceneComponent.K2_AddLocalOffset` _returnvalue (`KismetMathLibrary.MakeVector` 0.0 0.0 `_新規track_0`) false false))))))
        (:`Effect End`
          (`ActorComponent.K2_DestroyComponent` _returnvalue))
        (:`Effect Start2`
          (bind _returnvalue_2 (`GameplayStatics.SpawnEmitterAttached` "/Game/Effect/Effects_Boss/FANVFXCollection2/5_ParticleSystem/Barrier/Barrier_02/P_Barrier_02_05.P_Barrier_02_05" (`self.CapsuleComponent`) "None" (0.0 0.0 0.0) (struct) (5.0 5.0 5.0))))
        (:`Effect End2`
          (`ActorComponent.K2_DestroyComponent` _returnvalue_2))))))

(fn `CheckPlayerDIstance`
  (returns (approach :type Boolean))
  (if (< (`KismetMathLibrary.Vector_Distance` (`self.K2_GetActorLocation`) (`self.K2_GetActorLocation` (`GameplayStatics.GetPlayerPawn` 0))) (`self.distance`))
    (return true)
    (else
      (return false))))

(fn `GetNowPosition`
  (returns (position :type "/Game/BP/Boss/POSITION_NUM Enum"))
  (return (`self.NowDisPos`)))

(fn `RandAttackChoice`
  (returns (AttackNum :type Integer))
  (locals (AttackLoop :type Boolean :default true) (NowAttackNum :type Integer))
  (bind _lowattackcount (`self.LowAttackCount`))
  (bind _mediumattackcount (`self.MediumAttackCount`))
  (if (and (== (`self.LowAttackCount`) 2) (== (`self.MediumAttackCount`) 4))
    (set `self.LowAttackCount` 0)
    (set `self.MediumAttackCount` 0))
  (while (`local.AttackLoop`)
    (bind _output_get (set `local.NowAttackNum` (`KismetMathLibrary.RandomInteger` 3)))
    (if (!= _output_get (`self.PrevAttackNum`))
      (switch `int` (`local.NowAttackNum`)
        (:`0`
          (if (< _lowattackcount 2)
            (`/Engine/EditorBlueprintResources/StandardMacros.IncrementInt` _lowattackcount
              (:`  `
                (set `local.AttackLoop` false :!label _label)
                (set `self.PrevAttackNum` (`local.NowAttackNum`))))))
        (:`1`
          (if (< _mediumattackcount 4)
            (`/Engine/EditorBlueprintResources/StandardMacros.IncrementInt` _mediumattackcount
              (:`  `
                (goto _label)))))
        (:`2`
          (goto _label)))))
  (return (`local.NowAttackNum`)))

(fn `SetPlayerDistance`
  (bind _distance (`self.distance`))
  (set `self.distance` (`KismetMathLibrary.Vector_Distance` (`self.K2_GetActorLocation`) (`self.K2_GetActorLocation` (`GameplayStatics.GetPlayerPawn` 0))))
  (if (>= _distance 1800.0)
    (set `self.NowDisPos` "NewEnumerator2")
    (elif (and (< _distance 1800.0) (> _distance 800.0))
      (set `self.NowDisPos` "NewEnumerator1")
      (else
        (set `self.NowDisPos` "NewEnumerator0")))))

(fn `StartAttack`
  (`self.Attack`))

(fn `UserConstructionScript`)