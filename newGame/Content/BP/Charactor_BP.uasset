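; Player character Blueprint for melee combat, with movement, combo and charge attacks, guarding, health and death.
; Tick drives charge timing through a Gate, plus a guard meter that drains, regenerates and stuns on break.
; Hits resolve after a short frame-counted window, letting a right-click just guard negate damage, counterattack and copy the attacker's attribute.
; Left-click release advances a buffered MultiGate combo, and number keys switch attack attribute.
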(event `self.ReceiveAnyDamage`
  (params (Damage :type "Float (single-precision)") (DamageType :type "DamageType Object Reference") (InstigatedBy :type "Controller Object Reference") (DamageCauser :type "Actor Object Reference"))
  ;[1 1 1] Hit時
  (set `self.HitDamage` Damage)
  (set `self.Damage Causer` DamageCauser)
  (set `self.IsHit` true)
  (set `self.JastBlockTime` 0.0))

(event `Key|RightMouseButton`
  (params (Key :type "Key Structure"))
  ;[1 1 1] ガード処理
  (:`Pressed`
    (if (and (not (`self.IsAttacking`)) (not (`self.CanCombo`)) (not (`self.BlockBrake`)) (not (`self.RecoverFlag`)))
      (if (and (`self.IsHit`) (<= (`self.JastBlockTime`) (`self.MaxJastBlockTime`)))
        (set `self.JastBLock` true)
        (`KismetSystemLibrary.PrintString` "ジャストガード")
        ;;[1 1 1] ジャストガード後攻撃
        (bind _asenemy_bp (cast `/Game/BP/Enemy_BP` (`self.Damage Causer`)))
        (set `self.AttackState` (`/Game/BP/Enemy_BP.Attribute` _asenemy_bp))
        (`self.PlayAnimMontage` "/Game/BP/Combo_2.Combo_2" 1.0 "SecondSection")
        (set `self.invincibleTime` 0.0)
        (else
          (`self.BlockOpen`)
          (set `self.BlockFlag` true)
          (if (>= (`self.BlockTime`) 0.0)
            (`self.PlayAnimMontage` "/Game/BP/Block.Block" 0.1 "Default"))))))
  (:`Released`
    (`self.BLockClose`)
    (set `self.BlockFlag` false)
    (`self.StopAnimMontage` "/Game/BP/Block.Block")))

(event `BreakBlock`
  ;[1 1 1] ガード処理
  (`self.StopAnimMontage` "/Game/BP/Block.Block")
  (`self.BLockClose`)
  (set `self.BlockFlag` false))

(event `BlockOpen`
  ;[1 1 1] ガード処理
  (goto _label_3 :!via `Open`))

(event `self.ReceiveTick`
  (params (DeltaSeconds :type "Float (single-precision)"))
  (bind _jastblock (`self.JastBLock`))
  (if (not (`self.BlockBrake`))
    ;[1 1 1] ブレイク後Delay
    (if (`self.RecoverFlag`)
      (bind _output_get (set `self.RecoverDelay` (+ (`self.RecoverDelay`) DeltaSeconds)))
      (if (> _output_get 0.2)
        (set `self.RecoverFlag` false)
        (`|ExecutionSequence` :!label _label
          (:`then_0`
            ;[1 1 1] ガード処理
            (if (not (`self.BlockFlag`))
              (if (`self.EnemyDamegeFlag`)
                (set `self.BlockTime` (+ (`self.BlockTime`) (`self.BlockRecovePoint`)))
                (`KismetSystemLibrary.PrintString` "回復した")
                (set `self.EnemyDamegeFlag` false))
              ;;[1 1 1] ガード復活時間
              (bind _output_get_2 (set `self.BlockTime` (+ (`self.BlockTime`) DeltaSeconds)))
              (if (> _output_get_2 (`self.MaxBlockTime`))
                (set `self.BlockTime` (`self.MaxBlockTime`)))))
          (:`then_1`
            ;[1 1 1] コンボ攻撃
            (`/Engine/EditorBlueprintResources/StandardMacros.Gate` true :!label _label_2
              (:`Exit`
                (set `self.LoopPress` (- (`self.LoopPress`) (`GameplayStatics.GetWorldDeltaSeconds`)))
                (if (and (`self.BlockFlag`) (> (`KismetMathLibrary.Abs` (`self.LoopPress`)) (`self.MaxBlockTime`)))
                  _))))
          (:`then_2`
            (`/Engine/EditorBlueprintResources/StandardMacros.Gate` true :!label _label_3
              (:`Exit`
                (bind _output_get_3 (set `self.BlockTime` (- (`self.BlockTime`) (`GameplayStatics.GetWorldDeltaSeconds`))))
                (if (and (`self.BlockFlag`) (<= _output_get_3 0.0))
                  (`self.BreakBlock`)))))
          (:`then_3`
            (if (`self.IsHit`)
              (bind _result (`/Engine/EditorBlueprintResources/StandardMacros.IncrementFloat` (`self.JastBlockTime`))
                (:`  `
                  (`KismetSystemLibrary.PrintString` (`KismetStringLibrary.Conv_DoubleToString` _result))))))
          (:`then_4`
            ;[1 1 1] 攻撃を受けた場合の処理
            (if (and (> (`self.JastBlockTime`) (`self.MaxJastBlockTime`)) (`self.IsHit`))
              (set `self.IsHit` false)
              (set `self.JastBlockTime` 0.0)
              (if (or (`self.BlockFlag`) _jastblock)
                (if _jastblock
                  (set `self.JastBLock` false)
                  (`KismetSystemLibrary.PrintString` "ガードダメージなし")
                  (else
                    ;;[1 1 1] 攻撃ガード処理
                    (bind _output_get_4 (set `self.BlockTime` (- (`self.BlockTime`) 10.0)))
                    (if (<= _output_get_4 0.0)
                      (set `self.BlockBrake` true)
                      (set `self.BlockTime` 0.0)
                      (`KismetSystemLibrary.PrintString` "ガードブレイク")
                      (`self.BreakBlock`)
                      (`self.PlayAnimMontage` "/Game/RetergetAnim/Hit.Hit" 1.0 "Dafault")
                      (`CharacterMovementComponent.DisableMovement` (`self.CharacterMovement`)))))
                (else
                  (bind _output_get_5 (set `self.health` (- (`self.health`) (`self.HitDamage`))))
                  (if (> _output_get_5 0.0)
                    ;;[1 1 1] HPがまだ残っている状態
                    (`self.PlayAnimMontage` "/Game/RetergetAnim/Hit.Hit" 1.0 "Dafault")
                    (else
                      ;;[1 1 1] 死んだ時
                      (`/Engine/EditorBlueprintResources/StandardMacros.DoOnce` false
                        (:`Completed`
                          (bind _returnvalue (`self.PlayAnimMontage` null))
                          (`KismetSystemLibrary.Delay` (- _returnvalue 0.27))
                          (set `SkeletalMeshComponent.bPauseAnims` true (`self.Mesh`))
                          (`CharacterMovementComponent.DisableMovement` (`self.CharacterMovement`))))))))))))
      (else
        (goto _label)))
    (else
      ;[1 1 1] ガードブレイク状態
      (set `self.BLockBrakeTime` (+ DeltaSeconds (`self.BLockBrakeTime`)))
      (if (>= (`self.BLockBrakeTime`) (`self.MaxBlockBrakeTime`))
        (`CharacterMovementComponent.SetMovementMode` (`self.CharacterMovement`) "MOVE_Walking" 0)
        (set `self.BlockBrake` false)
        (set `self.BLockBrakeTime` 0.0)
        (`KismetSystemLibrary.PrintString` "ブレイク終了")
        (set `self.RecoverFlag` true)))))

(event `BLockClose`
  ;[1 1 1] ガード処理
  (goto _label_3 :!via `Close`))

(event `Open`
  ;[1 1 1] コンボ攻撃
  (goto _label_2 :!via `Open`))

(event `Close`
  ;[1 1 1] コンボ攻撃
  (goto _label_2 :!via `Close`))

(event `Key|LeftMouseButton`
  (params (Key :type "Key Structure"))
  ;[1 1 1] コンボ攻撃
  (:`Pressed`
    (set `self.LoopPress` 0.0)
    (`self.Open`))
  (:`Released`
    (if (and (not (`self.BlockBrake`)) (not (`self.BlockFlag`)) (not (`self.RecoverFlag`)))
      (`self.Close`)
      (if (> (`KismetMathLibrary.Abs` (`self.LoopPress`)) (`self.MaxChargeTime`))
        (set `self.ChargeAttackFlag` true)
        (else
          (set `self.ChargeAttackFlag` false)))
      (if (`self.IsAttacking`)
        (set `self.CanCombo` true)
        (else
          (set `self.IsAttacking` true)
          (`self.Attack`))))))

(event `Attack`
  (bind _chargeattackflag (`self.ChargeAttackFlag`))
  ;[1 1 1] コンボ攻撃
  (`CharacterMovementComponent.DisableMovement` (`self.CharacterMovement`))
  (`|MultiGate` false :!label _label_4
    (:`Out 0`
      (if _chargeattackflag
        (`self.PlayAnimMontage` "/Game/BP/ChargeAttack.ChargeAttack" 1.0 "FirstSection")
        (else
          (`self.PlayAnimMontage` "/Game/BP/Combo_2.Combo_2" 1.0 "FirstSection"))))
    (:`Out 1`
      (if _chargeattackflag
        (`self.PlayAnimMontage` "/Game/BP/ChargeAttack.ChargeAttack" 1.0 "FirstSection")
        (else
          (`self.PlayAnimMontage` "/Game/BP/Combo_2.Combo_2" 1.0 "SecondSection"))))
    (:`Out 2`
      (if _chargeattackflag
        (`self.PlayAnimMontage` "/Game/BP/ChargeAttack.ChargeAttack" 1.0 "FirstSection")
        (else
          (`self.PlayAnimMontage` "/Game/BP/Combo_2.Combo_2" 1.0 "ThirdSection"))))))

(event `Reset`
  ;[1 1 1] コンボ攻撃
  (goto _label_4 :!via `Reset`))

(event `SaveAttack`
  ;[1 1 1] コンボ攻撃
  (if (`self.CanCombo`)
    (set `self.CanCombo` false)
    (`self.Attack`)))

(event `Key|Zero`
  (params (Key :type "Key Structure"))
  ;[1 1 1] 武器変更
  (:`Pressed`
    (bind _output_get (set `self.AttackState` "NewEnumerator3"))
    (`KismetSystemLibrary.PrintString` (`|GetEnumeratorNameAsString` _output_get))))

(event `Key|One`
  (params (Key :type "Key Structure"))
  ;[1 1 1] 武器変更
  (:`Pressed`
    (bind _output_get (set `self.AttackState` "NewEnumerator5"))
    (`KismetSystemLibrary.PrintString` (`|GetEnumeratorNameAsString` _output_get))))

(event `ResetCombo`
  ;[1 1 1] コンボ攻撃
  (set `self.IsAttacking` false)
  (set `self.CanCombo` false)
  (`self.Reset`)
  (`CharacterMovementComponent.SetMovementMode` (`self.CharacterMovement`) "MOVE_Walking" 0))

(event `Key|Two`
  (params (Key :type "Key Structure"))
  ;[1 1 1] 武器変更
  (:`Pressed`
    (bind _output_get (set `self.AttackState` "NewEnumerator6"))
    (`KismetSystemLibrary.PrintString` (`|GetEnumeratorNameAsString` _output_get))))

(event `self.ReceiveBeginPlay`
  ;[1 1 1] 剣で自分がダメージを受けないようにする
  (`self.SetOwner` (`ChildActorComponent.ChildActor` (`self.ChildActor`)) self))

(event `InputAxis|Move Forward / Backward`
  (params (AxisValue :type "Float (single-precision)"))
  ;[1 1 1] 移動処理
  (`self.AddMovementInput` (`KismetMathLibrary.GetForwardVector` (`KismetMathLibrary.MakeRotator` 0.0 0.0 (.yaw (`self.GetControlRotation`)))) AxisValue))

(event `InputAxis|Turn Right / Left Mouse`
  (params (AxisValue :type "Float (single-precision)"))
  ;[1 1 1] 移動処理
  (`self.AddControllerYawInput` AxisValue))

(event `InputAxis|Look Up / Down Mouse`
  (params (AxisValue :type "Float (single-precision)"))
  ;[1 1 1] 移動処理
  (`self.AddControllerPitchInput` AxisValue))

(event `InputAction|Jump`
  (params (Key :type "Key Structure"))
  ;[1 1 1] 移動処理
  (:`Pressed`
    (`self.Jump`))
  (:`Released`
    (`self.StopJumping`)))

(event `InputAxis|Move Right / Left`
  (params (AxisValue :type "Float (single-precision)"))
  ;[1 1 1] 移動処理
  (`self.AddMovementInput` (`KismetMathLibrary.GetRightVector` (`KismetMathLibrary.MakeRotator` 0.0 0.0 (.yaw (`self.GetControlRotation`)))) AxisValue))

(fn `UserConstructionScript`)