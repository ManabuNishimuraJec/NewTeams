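; BP_doorBase is a key-locked door that disappears when the player holds its matching key.
; On any overlap with its Box, it reads the key list from player 0's Charactor_BP, without checking which actor overlapped.
; CheckKeyData compares each entry's KeyName with the door's own KeyData; a match sets that KeyData's boolean to true and the door destroys itself.
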(event `self.Box.OnComponentBeginOverlap`
  (params (OverlappedComponent :type "PrimitiveComponent Object Reference") (OtherActor :type "Actor Object Reference") (OtherComp :type "PrimitiveComponent Object Reference") (OtherBodyIndex :type Integer) (bFromSweep :type Boolean) (SweepResult :type "HitResult Structure (by ref)"))
  (bind _ascharactor_bp (cast `/Game/BP/Charactor_BP` (`GameplayStatics.GetPlayerCharacter` 0)))
  (bind _keydata (`/Game/BP/Charactor_BP.GetKeyData` _ascharactor_bp))
  (for _array_element _keydata
    (bind _match (`self.Check Key Data` _array_element))
    (if _match
      (`self.K2_DestroyActor`))))

(fn `Check Key Data`
  (params (PlayerKeyData :type "/Game/BP/Item/KeyData Structure"))
  (returns (Match :type Boolean))
  (bind _keyname (break `/Game/BP/Item/KeyData` (`self.KeyData`)))
  (if (== (`.KeyName_8_C9D1C83F451A1222C846FDA578940EBD` (break `/Game/BP/Item/KeyData` PlayerKeyData)) _keyname)
    (set `self.KeyData` (make `/Game/BP/Item/KeyData` _keyname true))
    (return true)
    (else
      (return false))))

(fn `UserConstructionScript`)