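; Base Blueprint for a sci-fi wing effect, rendered by a Niagara system through its User parameters.
; The construction script and Tick push the Scene component's world location and forward-derived rotation into Niagara.
; When EnbleFlying is set, a BeginPlay timeline flaps the wing by ping-ponging User.Angle within 0–1, stepped by frame delta.
; Setter functions expose shape and animation parameters, while a random-init chain is left unconnected.
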(event `self.ReceiveTick`
  (params (DeltaSeconds :type "Float (single-precision)"))
  (bind _niagara (`self.Niagara`))
  ;[1 0 0] This part is important, you should input the User.WingOrigin and User.WingRotation in here
  (set `self.DeltaSpeed` DeltaSeconds)
  (`/Engine/EditorBlueprintResources/StandardMacros.IsValid` _niagara
    (:`Is Valid`
      (`NiagaraComponent.SetNiagaraVariableVec3` _niagara "User.WingOrigin" (.location (`SceneComponent.K2_GetComponentToWorld` (`self.Scene`))))
      (`NiagaraComponent.SetNiagaraVariableQuat` (`self.Niagara`) "User.WingRotation" (`KismetMathLibrary.Conv_VectorToQuaterion` (`KismetMathLibrary.GetForwardVector` (`KismetMathLibrary.MakeRotator` 0.0 (.pitch (.rotation (`SceneComponent.K2_GetComponentToWorld` (`self.Scene`)))) (.yaw (.rotation (`SceneComponent.K2_GetComponentToWorld` (`self.Scene`)))))))))))

(event `self.ReceiveBeginPlay`
  (bind _niagara (`self.Niagara`))
  (bind _returnvalue (+ (`self.Speed`) (* (* (`self.SpeedCoefficient`) (`self.DeltaSpeed`)) (`self.SpeedFactor`))))
  (bind _returnvalue_2 (`KismetMathLibrary.Fraction` _returnvalue))
  ;[1 1 1] Wings waving logic
  (if (`self.EnbleFlying`)
    (`Timeline|Timeline_0` :`NewTime` 5.0
      (:`Update`
        (if (>= _returnvalue_2 0.95)
          (set `self.SpeedFactor` -1.0)
          (`NiagaraComponent.SetNiagaraVariableFloat` _niagara "User.Angle" _returnvalue_2)
          (set `self.Speed` _returnvalue)
          (elif (<= _returnvalue_2 0.05)
            (set `self.SpeedFactor` 1.0)
            (`NiagaraComponent.SetNiagaraVariableFloat` _niagara "User.Angle" _returnvalue_2)
            (set `self.Speed` _returnvalue)
            (else
              (`NiagaraComponent.SetNiagaraVariableFloat` _niagara "User.Angle" _returnvalue_2)
              (set `self.Speed` _returnvalue))))))))

(fn `Set Age Scale`
  (params (inputFloat :type "Float (double-precision)"))
  (`NiagaraComponent.SetNiagaraVariableFloat` (`self.Niagara`) "User.AgeScale" inputFloat))

(fn `Set Angle`
  (params (inputFloat :type "Float (double-precision)"))
  (`NiagaraComponent.SetNiagaraVariableFloat` (`self.Niagara`) "User.Angle" inputFloat))

(fn `Set Lightness`
  (params (inputFloat :type "Float (double-precision)"))
  (`NiagaraComponent.SetNiagaraVariableFloat` (`self.Niagara`) "User.Lightness" inputFloat))

(fn `Set MaxAmplitude`
  (params (inputFloat :type "Float (double-precision)"))
  (`NiagaraComponent.SetNiagaraVariableFloat` (`self.Niagara`) "User.MaxAmplitude" inputFloat))

(fn `Set MaxAnimationSpeed`
  (params (inputFloat :type "Float (double-precision)"))
  (`NiagaraComponent.SetNiagaraVariableFloat` (`self.Niagara`) "User.MaxAnimationSpeed" inputFloat))

(fn `Set MaxLength`
  (params (inputFloat :type "Float (double-precision)"))
  (`NiagaraComponent.SetNiagaraVariableFloat` (`self.Niagara`) "User.MaxLength" inputFloat))

(fn `Set MaxPeriod`
  (params (inputFloat :type "Float (double-precision)"))
  (`NiagaraComponent.SetNiagaraVariableFloat` (`self.Niagara`) "User.MaxPeriod" inputFloat))

(fn `Set MinAmplitude`
  (params (inputFloat :type "Float (double-precision)"))
  (`NiagaraComponent.SetNiagaraVariableFloat` (`self.Niagara`) "User.MinAmplitude" inputFloat))

(fn `Set MinAmplitudeSpeed`
  (params (inputFloat :type "Float (double-precision)"))
  (`NiagaraComponent.SetNiagaraVariableFloat` (`self.Niagara`) "User.MinAmplitudeSpeed" inputFloat))

(fn `Set MinLength`
  (params (inputFloat :type "Float (double-precision)"))
  (`NiagaraComponent.SetNiagaraVariableFloat` (`self.Niagara`) "User.MinLength" inputFloat))

(fn `Set MinPeriod`
  (params (inputFloat :type "Float (double-precision)"))
  (`NiagaraComponent.SetNiagaraVariableFloat` (`self.Niagara`) "User.MinPeriod" inputFloat))

(fn `Set Niagara Type`
  (`NiagaraComponent.SetAsset` (`self.Niagara`) null))

(fn `Set Seed`
  (params (inputFloat :type "Float (double-precision)"))
  (`NiagaraComponent.SetNiagaraVariableFloat` (`self.Niagara`) "User.Seed" inputFloat))

(fn `Set Soft`
  (params (inputFloat :type "Float (double-precision)"))
  (`NiagaraComponent.SetNiagaraVariableFloat` (`self.Niagara`) "User.Soft" inputFloat))

(fn `Set SpawnCount`
  (params (inputFloat :type "Float (double-precision)"))
  (`NiagaraComponent.SetNiagaraVariableInt` (`self.Niagara`) "User.SpawnCount" (`KismetMathLibrary.FTrunc` inputFloat)))

(fn `Set WidthScale`
  (params (inputFloat :type "Float (double-precision)"))
  (`NiagaraComponent.SetNiagaraVariableFloat` (`self.Niagara`) "User.WidthScale" inputFloat))

(fn `UserConstructionScript`
  (bind _niagara (`self.Niagara`))
  (`/Engine/EditorBlueprintResources/StandardMacros.IsValid` _niagara
    (:`Is Valid`
      (`NiagaraComponent.SetNiagaraVariableVec3` _niagara "WingOrigin" (.location (`SceneComponent.K2_GetComponentToWorld` (`self.Scene`))))
      (`NiagaraComponent.SetNiagaraVariableQuat` (`self.Niagara`) "User.WingRotation" (`KismetMathLibrary.Conv_VectorToQuaterion` (`KismetMathLibrary.GetForwardVector` (`KismetMathLibrary.MakeRotator` 0.0 (.pitch (.rotation (`SceneComponent.K2_GetComponentToWorld` (`self.Scene`)))) (.yaw (.rotation (`SceneComponent.K2_GetComponentToWorld` (`self.Scene`)))))))))))