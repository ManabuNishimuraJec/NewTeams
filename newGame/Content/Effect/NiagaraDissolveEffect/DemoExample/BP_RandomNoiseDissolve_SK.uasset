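; Demo actor that repeatedly plays a randomized noise dissolve with Niagara particles on an animated skeletal mesh.
; Each cycle picks a random emissive color and dissolve texture, shared by a dynamic mesh material and an attached Niagara system sampling the mesh.
; A timeline drives the material parameter collection's Amount and fades particle ForceIntensity, then restarts after a short delay.
; The particle scale setters are unconnected.
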(event `self.ReceiveBeginPlay`
  (bind _skeletalmesh (`self.SkeletalMesh`))
  ;[1 1 1] Dissolve Anim
  (`SceneComponent.SetVisibility` _skeletalmesh true false)
  (`SkeletalMeshComponent.PlayAnimation` _skeletalmesh (`self.Anim`) true)
  (bind _niagara (`self.SpawnNiagaraSystem` _skeletalmesh :!label _label))
  (`TimelineComponent.SetPlayRate` (`self.Timeline_0`) (`self.DissolveAnimRate`))
  (bind (_direction _newtrack_0) (`Timeline|Timeline_0` :!via `PlayFromStart`)
    (:`Update`
      (`KismetMaterialLibrary.SetScalarParameterValue` "/Game/Effect/NiagaraDissolveEffect/DemoRoom/SkeletalMeshExample/Character/Materials/Dissolve_RandomNoise/MPC_RandomNoiseDissolve_SK.MPC_RandomNoiseDissolve_SK" "Amount" _newtrack_0)
      (`NiagaraComponent.SetVariableFloat` _niagara "ForceIntensity" (`KismetMathLibrary.Lerp` (`self.ForceIntensity`) 0.0 _newtrack_0)))
    (:`Finished`
      (`KismetSystemLibrary.Delay` 1.0)
      (`ActorComponent.K2_DestroyComponent` _niagara)
      (goto _label))))

(fn `NiagaraSetting`
  (params (Niagara :type "NiagaraComponent Object Reference") (SpawnRate :type "Float (double-precision)") (NoiseFrequency :type "Float (double-precision)") (MinParticleScale :type "Float (double-precision)") (MaxParticleScale :type "Float (double-precision)"))
  ;[1 1 1] Setting NiagaraVariable
  (`NiagaraComponent.SetVariableFloat` Niagara "SpawnRate" SpawnRate)
  (`NiagaraComponent.SetVariableFloat` Niagara "NoiseFrequency" NoiseFrequency))

(fn `SpawnNiagaraSystem`
  (params (SkeletalMeshComponent :type "SkeletalMeshComponent Object Reference"))
  (returns (Niagara :type "NiagaraComponent Object Reference"))
  (locals (Color :type "LinearColor Structure") (TextureArray :type "Array of Texture Object Reference") (DissolveTexture :type "Texture Object Reference") (MI :type "MaterialInstanceDynamic Object Reference") (M_Niagara :type "MaterialInterface Object Reference" :default "Material'/Game/Effect/NiagaraDissolveEffect/DemoRoom/SkeletalMeshExample/Character/Materials/Dissolve_RandomNoise/M_Male_Body_Niagara.M_Male_Body_Niagara'"))
  (set `local.Color` (* (make `LinearColor` (`KismetMathLibrary.RandomFloatInRange` 0.0 1.0) (`KismetMathLibrary.RandomFloatInRange` 0.0 1.0) (`KismetMathLibrary.RandomFloatInRange` 0.0 1.0) 1.0) 100.0))
  (set `local.DissolveTexture` (`|GetArrayItem` (`local.TextureArray`) (`KismetMathLibrary.RandomIntegerInRange` 0 2)))
  ;[1 1 1] Set Random Dissolve Effect
  (bind _returnvalue (`PrimitiveComponent.CreateDynamicMaterialInstance` SkeletalMeshComponent 0 null "None"))
  (`MaterialInstanceDynamic.SetTextureParameterValue` _returnvalue "DissolveTexture" (`local.DissolveTexture`))
  (`MaterialInstanceDynamic.SetVectorParameterValue` _returnvalue "EmissiveColor" (`local.Color`))
  (bind _returnvalue_2 (`KismetMaterialLibrary.CreateDynamicMaterialInstance` (`local.M_Niagara`)))
  (bind _output_get (set `local.MI` _returnvalue_2))
  (`MaterialInstanceDynamic.SetTextureParameterValue` _returnvalue_2 "DissolveTexture" (`local.DissolveTexture`))
  (bind _returnvalue_3 (`NiagaraFunctionLibrary.SpawnSystemAttached` "/Game/Effect/NiagaraDissolveEffect/Niagara/P_RandomNoiseDissolve_SK.P_RandomNoiseDissolve_SK" SkeletalMeshComponent "None" (0.0 0.0 0.0) (struct) "KeepRelativeOffset" true))
  (`NiagaraComponent.SetVariableMaterial` _returnvalue_3 "Material Interface" _output_get)
  (`NiagaraFunctionLibrary.OverrideSystemUserVariableSkeletalMeshComponent` _returnvalue_3 "Skeketal Mesh" SkeletalMeshComponent)
  (`NiagaraComponent.SetVariableVec3` _returnvalue_3 "EmissiveColor" (`KismetMathLibrary.Conv_LinearColorToVector` (`local.Color`)))
  (`self.NiagaraSetting` _returnvalue_3 (`self.Spawn Rate`) (`self.Noise Frequency`) (`self.Min Particle Scale`) (`self.Max Particle Scale`))
  (return _returnvalue_3))

(fn `UserConstructionScript`)